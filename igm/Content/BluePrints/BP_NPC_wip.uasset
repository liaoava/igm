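; Work-in-progress NPC Blueprint for killable wedding-style characters such as the groom, mother-in-law, brother, chef and teacher.
; On BeginPlay, the NPC name selects which character component to make visible, so one Blueprint covers every role.
; Kill passes that name to the first-person character as TargetName, increments its kill count, plays a sound and destroys the actor.
; The KillSphere overlap event has no logic, and a death animation remains only a noted idea.
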(event OnComponentBeginOverlap(KillSphere)
  (params (OverlappedComponent :type Primitive%20Component%20Object%20Reference) (OtherActor :type Actor%20Object%20Reference) (OtherComp :type Primitive%20Component%20Object%20Reference) (OtherBodyIndex :type Integer) (bFromSweep :type Boolean) (SweepResult :type Hit%20Result%20Structure%20%28by%20ref%29)))

(event EventBeginPlay
  (if (Utilities|Enum|Equal(Enum) (Variables|Default|GetNPC) "Groom")
    (Rendering|SetVisibility (Variables|Default|GetGroom) true false)
    (elif (Utilities|Enum|Equal(Enum) (Variables|Default|GetNPC) "MIL")
      (Rendering|SetVisibility (Variables|Default|GetMother) true false)
      (elif (Utilities|Enum|Equal(Enum) (Variables|Default|GetNPC) "Brother")
        (Rendering|SetVisibility (Variables|Default|GetBrother) true false)
        (elif (Utilities|Enum|Equal(Enum) (Variables|Default|GetNPC) "Chef")
          (Rendering|SetVisibility (Variables|Default|GetChef) true true)
          (elif (Utilities|Enum|Equal(Enum) (Variables|Default|GetNPC) "Teacher")
            (Rendering|SetVisibility (Variables|Default|GetTeacher) true false)))))))

(event EventKill
  (bind _npc (Variables|Default|GetNPC))
  (bind _asfirst_person_character (Utilities|Casting|CastToFirstPersonCharacter (stale OnComponentBeginOverlap(KillSphere) OtherActor)))
  (Variables|/Game/FirstPersonBP/Blueprints/FirstPersonCharacter.FirstPersonCharacter_C|SetTargetName _asfirst_person_character _npc)
  (Development|PrintString _npc)
  (bind _result (Math|Integer|IncrementInt (Variables|/Game/FirstPersonBP/Blueprints/FirstPersonCharacter.FirstPersonCharacter_C|GetNumberofKills _asfirst_person_character))
    (:%20%20
      (Development|PrintString (Utilities|String|ToString(Integer) _result))
      (Audio|PlaySoundatLocation "/Game/FirstPerson/Audio/FirstPersonTemplateWeaponFire02.FirstPersonTemplateWeaponFire02" "0, 0, 0" "0, 0, 0" 1.0 1.0 0.0 0 0 0)
      ;[1 1 1] Instead of "Destroy actor" maybe we will want to play a death animation & turn off collission
      (Actor|DestroyActor))))

(fn ConstructionScript)