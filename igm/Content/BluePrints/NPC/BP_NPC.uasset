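; BP_NPC is a named character that flees the player and can be killed.
; BeginPlay shows the mesh matching its NPC name, caches the player character and starts RunAway.
; RunAway loops AI MoveTo toward random reachable points around a spot directly away from the player, retrying on success or failure.
; Kill passes the name to the player, increments the kill count, plays a sound and destroys the NPC.
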(event OnComponentBeginOverlap(KillSphere)
  (params (OverlappedComponent :type Primitive%20Component%20Object%20Reference) (OtherActor :type Actor%20Object%20Reference) (OtherComp :type Primitive%20Component%20Object%20Reference) (OtherBodyIndex :type Integer) (bFromSweep :type Boolean) (SweepResult :type Hit%20Result%20Structure%20%28by%20ref%29)))

(event Custom|RunAway
  (bind _returnvalue (Transformation|GetActorLocation))
  (bind _char_ref (Variables|Default|GetChar%20REF))
  (bind _returnvalue_2 (Transformation|GetActorLocation _char_ref))
  (bind _returnvalue_3 (Math|Rotator|FindLookatRotation _returnvalue _returnvalue_2))
  (bind _returnvalue_4 (Math|Vector|GetForwardVector _returnvalue_3))
  (bind _returnvalue_5 (* _returnvalue_4 -5e+02))
  (bind _returnvalue_6 (+ _returnvalue _returnvalue_5))
  (bind (_x _y) (Math|Vector|BreakVector _returnvalue_6))
  (AI|AIMoveTo self (.RandomLocation (AI|Navigation|GetRandomReachablePointinRadius (Math|Vector|MakeVector _x _y (.Z (Math|Vector|BreakVector _returnvalue))) 5e+02 0 0)) 0 5.0 false
    (:OnSuccess
      _)
    (:OnFail
      _))
  (CallFunction|RunAway))

(event EventBeginPlay
  (Utilities|FlowControl|Sequence
    (:then_0
      ;[1 1 1] Sets mesh based off NPC name
      (if (Utilities|Enum|Equal(Enum) (Variables|Default|GetNPC) "Groom")
        (Rendering|SetVisibility (Variables|Default|GetGroom) true false)
        (elif (Utilities|Enum|Equal(Enum) (Variables|Default|GetNPC) "MIL")
          (Rendering|SetVisibility (Variables|Default|GetMother) true false)
          (elif (Utilities|Enum|Equal(Enum) (Variables|Default|GetNPC) "Brother")
            (Rendering|SetVisibility (Variables|Default|GetBrother) true false)
            (elif (Utilities|Enum|Equal(Enum) (Variables|Default|GetNPC) "Chef")
              (Rendering|SetVisibility (Variables|Default|GetChef) true true)
              (elif (Utilities|Enum|Equal(Enum) (Variables|Default|GetNPC) "Teacher")
                (Rendering|SetVisibility (Variables|Default|GetTeacher) true false)))))))
    (:then_1
      (bind _asfirst_person_character (Utilities|Casting|CastToFirstPersonCharacter (Game|GetPlayerCharacter 0)))
      (Variables|Default|SetChar%20REF _asfirst_person_character)
      (CallFunction|RunAway))))

(event EventKill
  (bind _npc (Variables|Default|GetNPC))
  (bind _asfirst_person_character (Utilities|Casting|CastToFirstPersonCharacter (stale OnComponentBeginOverlap(KillSphere) OtherActor)))
  (Variables|/Game/FirstPersonBP/Blueprints/FirstPersonCharacter.FirstPersonCharacter_C|SetTargetName _asfirst_person_character _npc)
  (Development|PrintString _npc)
  (bind _result (Math|Integer|IncrementInt (Variables|/Game/FirstPersonBP/Blueprints/FirstPersonCharacter.FirstPersonCharacter_C|GetNumberofKills _asfirst_person_character))
    (:%20%20
      (Development|PrintString (Utilities|String|ToString(Integer) _result))
      (Audio|PlaySoundatLocation "/Game/FirstPerson/Audio/FirstPersonTemplateWeaponFire02.FirstPersonTemplateWeaponFire02" "0, 0, 0" "0, 0, 0" 1.0 1.0 0.0 0 0 0)
      ;[1 1 1] Instead of "Destroy actor" maybe we will want to play a death animation & turn off collission
      (Actor|DestroyActor))))

(fn ConstructionScript)