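; Weapon pickup actor that equips its weapon on the FirstPersonCharacter when that character overlaps its Box.
; It loops over the character's WeaponMeshes, showing the one whose object name matches WeaponName and hiding the rest.
; On a match it stores its own class as ActiveWeapon and destroys itself.
; Socket-attach and static-mesh-swap alternatives remain in the graph but are disconnected.
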(event OnComponentBeginOverlap(Box)
  (params (OverlappedComponent :type Primitive%20Component%20Object%20Reference) (OtherActor :type Actor%20Object%20Reference) (OtherComp :type Primitive%20Component%20Object%20Reference) (OtherBodyIndex :type Integer) (bFromSweep :type Boolean) (SweepResult :type Hit%20Result%20Structure%20%28by%20ref%29))
  (Utilities|Casting|CastToFirstPersonCharacter OtherActor)
  ;[1 1 1] Setting mesh visibility way
  (bind _array_element (Utilities|Array|ForEachLoopwithBreak (Variables|/Game/FirstPersonBP/Blueprints/FirstPersonCharacter.FirstPersonCharacter_C|GetWeaponMeshes (Variables|Default|GetFirst%20Person%20Character)))
    (:LoopBody
      (if (Utilities|Enum|Equal(Enum) (Variables|Default|GetWeaponName) (Utilities|Text|ToText(String) (Utilities|GetObjectName _array_element)))
        (Rendering|SetVisibility _array_element true false)
        (Variables|/Game/FirstPersonBP/Blueprints/FirstPersonCharacter.FirstPersonCharacter_C|SetActiveWeapon (Variables|Default|GetFirst%20Person%20Character) (Utilities|GetClass self))
        (Actor|DestroyActor)
        (else
          (Rendering|SetVisibility _array_element false false))))))

(event EventBeginPlay
  (bind _asfirst_person_character (Utilities|Casting|CastToFirstPersonCharacter (Game|GetPlayerCharacter 0)))
  (Variables|Default|SetFirst%20Person%20Character _asfirst_person_character))

(event Collision|EventActorBeginOverlap
  (params (OtherActor :type Actor%20Object%20Reference)))

(event EventTick
  (params (DeltaSeconds :type Float%20%28single-precision%29)))

(fn ConstructionScript)